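; BP_Repairkit_Wpn is a weapon repair kit item that decides whether it can be dropped on a target item to repair it.
; CanBeDroppedOnItem silently rejects items already in repair, then refuses three hardcoded template IDs and items whose durability is not below their post-penalty maximum, showing a notification for both refusals.
; A rune-enchantment check against WeaponModkitTable is disconnected, so enchanted items are not blocked.
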(fn `CanBeDroppedOnItem`
  (params (TargetItem :type "GameItem Object Reference"))
  (returns (ReturnValue :type Boolean))
  (locals (LocalItem :type "GameItem Object Reference"))
  (bind _localitem (`local.LocalItem`))
  (bind _templateid (`GameItem.TemplateID` (`local.LocalItem`)))
  (set `local.LocalItem` TargetItem)
  (if (`self.GetIsInRepairState` (`local.LocalItem`))
    (return false)
    (else
      (if (!= (`self.GetIntStat` (`local.LocalItem`) "CurrentEnchantID") 0)
        _
        (else
          _))
      (if (and (not (== _templateid 51468)) (not (== _templateid 51545)) (not (== _templateid 50592)))
        (if (< (`self.GetFloatStat` _localitem "CurrentDurability") (`self.GetMaxDurabilityAfterPenalty` _localitem))
          (return true)
          (else
            (`self.ShowNotification` (`/Game/Items/Weapons/ItemFunctionLibrary.GetCannotDropReasonText` "NewEnumerator8") (`local.LocalItem`))
            (return false)))
        (else
          (`self.ShowNotification` (`/Game/Items/Weapons/ItemFunctionLibrary.GetCannotDropReasonText` "NewEnumerator6") (`local.LocalItem`))
          (return false))))))